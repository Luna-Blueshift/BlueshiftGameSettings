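; Game setting Blueprint for the color vision deficiency (colorblind) mode option.
; It offers Normal, Deuteranope, Protanope and Tritanope choices mapped to integer keys.
; Reading and writing go through BlueshiftGameUserSettings, converting the integer to the deficiency enum and updating color vision immediately on set.
; GetValue falls back to the parent value if the user settings cast fails.
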(event `self.SetValue`
  (params (Value :type Integer))
  (bind _returnvalue (`GameUserSettings.GetGameUserSettings`))
  (bind _asblueshift_game_user_settings (cast `BlueshiftGameUserSettings` _returnvalue))
  (`BlueshiftGameUserSettings.SetColorVisionDeficiencyMode` _asblueshift_game_user_settings (cast `EColorVisionDeficiency` (`KismetMathLibrary.Conv_IntToByte` Value)) true))

(fn `GetOptions`
  (returns (ReturnValue :type "Map of Integer to Text"))
  (return (`|MakeMap` 0 "Normal" 1 "Deuteranope" 2 "Protanope" 3 "Tritanope" :!valuetype "Text")))

(fn `GetValue`
  (returns (ReturnValue :type Integer))
  (bind _returnvalue (`GameUserSettings.GetGameUserSettings`))
  (bind _asblueshift_game_user_settings (cast `BlueshiftGameUserSettings` _returnvalue)
    (:`then`
      (return (`KismetMathLibrary.Conv_ByteToInt` (`BlueshiftGameUserSettings.GetColorVisionDeficiencyMode` _asblueshift_game_user_settings))))
    (:`CastFailed`
      (return (`parent.GetValue`)))))