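; Game setting Blueprint for the window mode option, covering Fullscreen, Windowed Fullscreen and Windowed.
; GetOptions maps every EWindowMode value to a display label, keyed by its integer.
; GetValue and SetValue read and write the fullscreen mode on GameUserSettings, converting between integer and enum.
; SetValue only sets the mode; the apply-resolution and temporary confirm-video-mode calls are disconnected and never run.
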(event `self.SetValue`
  (params (Value :type Integer))
  (bind _returnvalue (`GameUserSettings.GetGameUserSettings`))
  (`GameUserSettings.SetFullscreenMode` _returnvalue (cast `EWindowMode` (`KismetMathLibrary.Conv_IntToByte` Value))))

(fn `GetOptions`
  (returns (ReturnValue :type "Map of Integer to Text"))
  (locals (Result :type "Map of Integer to Text"))
  (bind _enumvalue (foreach `EWindowMode` false)
    (:`LoopBody`
      (`BlueprintMapLibrary.Map_Add` (`local.Result`) (`KismetMathLibrary.Conv_ByteToInt` _enumvalue) (select `EWindowMode` _enumvalue :`Fullscreen` "Fullscreen" :`WindowedFullscreen` "Windowed Fullscreen" :`Windowed` "Windowed")))
    (:`then`
      (return (`local.Result`)))))

(fn `GetValue`
  (returns (ReturnValue :type Integer))
  (bind _returnvalue (`GameUserSettings.GetGameUserSettings`))
  (return (`KismetMathLibrary.Conv_ByteToInt` (cast `EWindowMode` (`GameUserSettings.GetFullscreenMode` _returnvalue)))))