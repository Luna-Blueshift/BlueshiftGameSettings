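; Game setting for resolution scale, backed by GameUserSettings and shown as a percentage.
; SetValue calls the parent, then writes the value as a normalized resolution scale, while GetValue reads the non-normalized CurrentScaleValue.
; The declared float range is shown by multiplying by 100 and appending a percent sign, and GetDisplayValue returns an empty string.
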(event `self.SetValue`
  (params (Value :type "Float (single-precision)"))
  (`parent.SetValue` Value)
  (bind _returnvalue (`GameUserSettings.GetGameUserSettings`))
  (`GameUserSettings.SetResolutionScaleNormalized` _returnvalue Value))

(fn `GetDisplayValue`
  (returns (ReturnValue :type Text))
  (return ""))

(fn `GetDisplayValueFromFloat`
  (params (Value :type "Float (single-precision)"))
  (returns (ReturnValue :type Text))
  (return (`|FormatText` "{Resolution} %" (`KismetTextLibrary.Conv_DoubleToText` (* Value 100.0) "HalfToEven" false true 1 324 0 2))))

(fn `GetValue`
  (returns (ReturnValue :type "Float (single-precision)"))
  (bind _returnvalue (`GameUserSettings.GetGameUserSettings`))
  (return (`.CurrentScaleValue` (`GameUserSettings.GetResolutionScaleInformationEx` _returnvalue))))

(fn `GetValueRange`
  (returns (Min :type "Float (single-precision)") (Max :type "Float (single-precision)"))
  (return 0.0 2.0))