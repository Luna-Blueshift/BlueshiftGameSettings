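; BP_GameSetting_HDR is a game setting Blueprint that toggles HDR display output through Game User Settings.
; SetValue enables or disables HDR output at a fixed nits level, and GetValue reports whether HDR is currently enabled.
; GetVisibility returns Enabled only when the display output supports HDR, otherwise Disabled.
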(event `self.SetValue`
  (params (Value :type Boolean))
  (bind _returnvalue (`GameUserSettings.GetGameUserSettings`))
  (`GameUserSettings.EnableHDRDisplayOutput` _returnvalue Value 1000))

(fn `GetValue`
  (returns (ReturnValue :type Boolean))
  (bind _returnvalue (`GameUserSettings.GetGameUserSettings`))
  (return (`GameUserSettings.IsHDREnabled` _returnvalue)))

(fn `GetVisibility`
  (returns (ReturnValue :type "EBlueshiftGameSettingVisibility Enum"))
  (bind _returnvalue (`GameUserSettings.GetGameUserSettings`))
  (return (select `bool` (`GameUserSettings.SupportsHDRDisplayOutput` _returnvalue) :`false` "Disabled" :`true` "Enabled" :!type "EBlueshiftGameSettingVisibility Enum")))